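; BP_AI is a team deathmatch AI soldier that roams, hunts enemy pawns and fires a rifle at them.
; Random-point AIMoveTo drives searching until PawnSensing spots another team's pawn via BPI_TeamINteraction, then it chases and fires.
; A montage notify triggers effects and a damaging sphere trace from the muzzle.
; Death ragdolls it and updates GS_TeamDeathMatch's count, while Tick refreshes health and turns widgets toward the camera.
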(event OnSeePawn(PawnSensing)
  (params (Pawn :type Pawn%20Object%20Reference))
  (if (Utilities|DoesObjectImplementInterface Pawn "/Game/Blueprints/BPI_TeamINteraction.BPI_TeamINteraction_C")
    (bind _team (Class|BPITeamINteraction|GetTeam(Message) Pawn))
    (if (!= _team (Math|Conversions|ToInteger(Byte) (Variables|Default|Getteam)))
      (bind _asbp_ai (Utilities|Casting|CastToBP_AI Pawn)
        (:then
          (if (Variables|BP_AI_C|GetisDead? _asbp_ai)
            (CallFunction|SearchAround)
            (else
              (CallFunction|ChaseTarget Pawn :!label _label)
              (Variables|Default|SethasSeenTarget true))))
        (:CastFailed
          (goto _label))))))

(event Custom|Search%20Around
  ;[0.05098 0.05098 0.05098] Search Around
  (if (not (Variables|Default|GethasSeenTarget))
    (AI|AIMoveTo self (.RandomLocation (AI|Navigation|GetRandomReachablePointinRadius (Transformation|GetActorLocation) 2e+03 0 0)) 0 3e+02 false
      (:OnSuccess
        (Utilities|FlowControl|Delay 0.1)
        (CallFunction|SearchAround)))))

(event Custom|Chase%20Target
  (params (TargetActor :type Actor%20Object%20Reference))
  (AI|AIMoveTo self "0, 0, 0" TargetActor 5e+02 false
    (:OnSuccess
      (CallFunction|Fire TargetActor))))

(event Custom|Fire
  (params (Target%20Actor :type Actor%20Object%20Reference))
  (bind _mesh (Variables|Character|GetMesh))
  (bind _rifle (Variables|Default|Getrifle))
  (bind _returnvalue (Transformation|GetSocketTransform _rifle "b_gun_muzzleflash" "RTS_World"))
  (bind _returnvalue_2 (Transformation|GetWorldRotation _mesh))
  (if (not (Variables|Default|GetisDead?))
    (Pawn|SetControlRotation (Pawn|GetController) (Math|Rotator|FindLookatRotation (Transformation|GetActorLocation) (Transformation|GetActorLocation Target%20Actor)))
    (Animation|Montage|PlayMontage (Variables|Character|GetMesh) "/Game/anim/Fire_Rifle_shoot_Montage.Fire_Rifle_shoot_Montage"
      (:OnNotifyBegin
        (Effects|SpawnEmitterAttached "/Game/InfinityBladeEffects/Effects/FX_Monsters/FX_Monster_Gruntling/Master/P_BackPack_MuzzleFlash.P_BackPack_MuzzleFlash" (Variables|Default|Getrifle) "b_gun_muzzleflash" (.location _returnvalue) _returnvalue_2 "0.150000,0.150000,0.150000" "KeepWorldPosition" true "AutoRelease")
        (Audio|PlaySoundatLocation "/Game/Audio/MS_rifle.MS_rifle" (Transformation|GetActorLocation) "0, 0, 0" 0.6 1.0 0.0 0 0 0 0)
        (bind (_outhit _returnvalue_3) (Collision|SphereTraceByChannel (.location _returnvalue) (+ (.location _returnvalue) (* (Math|Vector|GetRightVector _returnvalue_2) 3e+03)) 12.0 "TraceTypeQuery1" false 0 "None"))
        (if _returnvalue_3
          (Game|Damage|ApplyDamage (.HitActor (Collision|BreakHitResult _outhit)) 5.0 0 0)
          (Effects|SpawnEmitteratLocation "/Game/InfinityBladeEffects/Effects/FX_Monsters/FX_Monster_Troll/death/P_TrollDeathImpact.P_TrollDeathImpact" (.ImpactPoint (Collision|BreakHitResult _outhit)) (Math|Rotator|MakeRotfromX (.Normal (Collision|BreakHitResult _outhit))) "0.500000,0.600000,0.500000")
          (Audio|PlaySoundatLocation "/Game/Audio/MS_hitconcrete.MS_hitconcrete" (Transformation|GetActorLocation) "0, 0, 0" 2.0 1.0 0.0 0 0 0 0))))))

(event EventTick
  (params (DeltaSeconds :type Float%20%28single-precision%29))
  (bind _asai_health_bar (Utilities|Casting|CastToAI_healthBAr (UserInterface|GetWidget (Variables|Default|Gethealth%20bar%20widget))))
  (Progress|SetPercent (Variables|/Game/AI_healthBAr.AI_healthBAr_C|GetHealthbar _asai_health_bar) (/ (Variables|Default|GetHealth) 1e+02))
  (Transformation|SetWorldRotation (Variables|Default|Gethealth%20bar%20widget) (Math|Rotator|FindLookatRotation (Transformation|GetActorLocation) (Transformation|GetActorLocation (Game|GetPlayerCameraManager 0))) false false))

(event EventBeginPlay
  (CallFunction|SearchAround)
  (Utilities|FlowControl|Sequence
    (:then_0
      (if (== (Variables|Default|Getteam) 1)
        (bind _asai_team (Utilities|Casting|CastToAI_team (UserInterface|GetWidget (Variables|Default|GetTeam%20Widget))))
        (Rendering|Components|TextRender|SetText (Variables|/Game/AI_team.AI_team_C|GetTeamTExt _asai_team) "TEAM B")
        (Appearance|SetColorandOpacity (Variables|/Game/AI_team.AI_team_C|GetTeamTExt _asai_team) (Utilities|Struct|MakeSlateColor "(R=0.593750,G=0.000000,B=0.010401,A=1.000000)") :!class /Script/UMG.TextBlock)
        (Class|TextBlock|SetFont (Variables|/Game/AI_team.AI_team_C|GetTeamTExt _asai_team) (Utilities|Struct|MakeSlateFontInfo "/Engine/EngineFonts/Roboto.Roboto" 0 (Utilities|Struct|MakeFontOutlineSettings 3 false false 0 "(R=0.171875,G=0.000000,B=0.000000,A=1.000000)") "Bold" 27))))
    (:then_1
      (Utilities|FlowControl|Delay 0.25 :!label _label)
      (if (Variables|Default|GethasSeenTarget)
        (CallFunction|SearchAround)
        (Variables|Default|SethasSeenTarget true)
        (goto _label)))))

(event Game|Damage|EventAnyDamage
  (params (Damage :type Float%20%28single-precision%29) (DamageType :type Damage%20Type%20Object%20Reference) (InstigatedBy :type Controller%20Object%20Reference) (DamageCauser :type Actor%20Object%20Reference))
  ;[0.05098 0.05098 0.05098] HEALTH and DAMAGE
  (Variables|Default|SetHealth (- (Variables|Default|GetHealth) Damage))
  (if (<= (Variables|Default|GetHealth) 0.0)
    (Utilities|FlowControl|DoOnce false
      (:Completed
        (Physics|SetSimulatePhysics (Variables|Character|GetMesh) true)
        (Pawn|Components|CharacterMovement|SetMovementMode (Variables|Character|GetCharacterMovement) "MOVE_None" 0)
        (Variables|Default|SetisDead? true)
        (Rendering|SetVisibility (Variables|Default|Gethealth%20bar%20widget) false false)
        (bind _asgs_team_death_match (Utilities|Casting|CastToGS_TeamDeathMatch (Game|GetGameState)))
        (Default|DecreaseTeamNumber _asgs_team_death_match (== (Variables|Default|Getteam) 0))))))

(event EventSetTeam
  (params (Team :type E_teams%20Enum :default "NewEnumerator0"))
  (Variables|Default|Setteam Team))

(fn ConstructionScript)

(fn GetTeam
  (return (Variables|Default|Getteam)))